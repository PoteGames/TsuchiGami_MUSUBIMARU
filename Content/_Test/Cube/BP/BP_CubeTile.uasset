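; BP_CubeTile is a test cube tile that, on MoveCube, moves vertically through start, wait and end timelines scaled by MoveRate.
; During the start phase it enlarges its box collision and enables a capsule query that collects overlapping "Enemy" actors.
; Hit stop briefly dilates the tile's time using BP_Default_Setting values, then messages collected enemies after the delay.
; A separate CubeHitEnemy event applies only the hit stop.
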(event OnComponentBeginOverlap(Capsule)
  (params (OverlappedComponent :type Primitive%20Component%20Object%20Reference) (OtherActor :type Actor%20Object%20Reference) (OtherComp :type Primitive%20Component%20Object%20Reference) (OtherBodyIndex :type Integer) (bFromSweep :type Boolean) (SweepResult :type Hit%20Result%20Structure%20%28by%20ref%29))
  (if (Utilities|IsValid OtherActor)
    (if (Actor|ActorHasTag OtherActor "Enemy")
      (Utilities|Array|AddUnique (Variables|Default|GetTarget_Enemy) OtherActor))))

(event Custom|HIt_Enemy
  (Variables|Default|SetCustomTimeDilation (Variables|Default|GetHit%20Stop%20Time%20Dilation))
  (Utilities|FlowControl|Delay (Variables|Default|GetHit%20Stop%20Delay))
  (Variables|Default|SetCustomTimeDilation 1.0)
  (for _array_element (Variables|Default|GetTarget_Enemy)
    (Class|BPIFCubeData|CubeHitEnemy(Message) _array_element self false)))

(event EventBeginPlay
  ;[0.15 0.15 0.15 0.5] 基本設定読み込み
  (bind _returnvalue (Actor|GetActorOfClass "/Game/_Test/BP_Default_Setting.BP_Default_Setting_C"))
  (Variables|Default|SetHit%20Stop%20Time%20Dilation (Variables|/Game/_Test/BP_Default_Setting.BP_Default_Setting_C|GetHitStop_TimeDilation _returnvalue))
  (Variables|Default|SetHit%20Stop%20Delay (Variables|/Game/_Test/BP_Default_Setting.BP_Default_Setting_C|GetHitStopDelay _returnvalue))
  (Class|BPIFCubeData|CubeTLStartLength(Message) _returnvalue (Components|Timeline|GetTimelineLength (Variables|Default|GetCube_TL_Start))))

(event EventMoveCube
  (params (MoveRate :type Float%20%28double-precision%29))
  (bind _max_move (Variables|Default|GetMax_Move))
  (bind _returnvalue (* _max_move MoveRate))
  (Utilities|Array|Clear (Variables|Default|GetTarget_Enemy))
  (Variables|Default|SetBox_Col_Size (Variables|/Script/Engine.BoxComponent|GetBoxExtent (Variables|Default|GetBox_Col)))
  (if (not (Variables|Default|GetRun_Animation))
    (Utilities|FlowControl|Sequence
      (:then_0
        (Components|Timeline|SetPlayRate (Variables|Default|GetCube_TL_Start) (Variables|Default|GetTL_Start_Rate)) ; スピード調節
        (Components|Timeline|SetPlayRate (Variables|Default|GetCube_TL_Wait) (Variables|Default|GetTL_Wait_Rate)) ; スピード調節
        (Components|Timeline|SetPlayRate (Variables|Default|GetCube_TL_End) (Variables|Default|GetTL_End_Rate)) ; スピード調節
      )
      (:then_1
        (Variables|Default|SetRun_Animation true)
        (Variables|Default|SetGet_Location (.location (Transformation|GetActorTransform)))
        (Components|Box|SetBoxExtent (Variables|Default|GetBox_Col) (* (Variables|Default|GetBox_Col_Size) "3.000000,3.000000,1.000000") true)
        (Variables|/Script/Engine.PrimitiveComponent|SetCanCharacterStepUpOn (Variables|Default|GetBox_Col) "ECB_No")
        (Collision|SetCollisionEnabled (Variables|Default|GetCapsule) "QueryOnly")
        (CallFunction|HItEnemy)
        (bind _move_curve_start (Timeline|Cube_TL_Start PlayFromStart)
          (:Update
            (Transformation|SetActorLocation (Math|Vector|MakeVector (.x (Variables|Default|GetGet_Location)) (.y (Variables|Default|GetGet_Location)) (Math|Float|Clamp(Float) (+ (.z (Variables|Default|GetGet_Location)) (* _returnvalue _move_curve_start)) 0.0 (Variables|Default|GetMax_Move))) false false))
          (:Finished
            (Collision|SetCollisionEnabled (Variables|Default|GetCapsule) "NoCollision")
            (Components|Box|SetBoxExtent (Variables|Default|GetBox_Col) (Variables|Default|GetBox_Col_Size) true)
            (bind _move_curve_wait (Timeline|Cube_TL_Wait PlayFromStart)
              (:Update
                (Transformation|SetActorLocation (Math|Vector|MakeVector (.x (Variables|Default|GetGet_Location)) (.y (Variables|Default|GetGet_Location)) (Math|Float|Clamp(Float) (+ (.z (Variables|Default|GetGet_Location)) (* _returnvalue _move_curve_wait)) 0.0 (Variables|Default|GetMax_Move))) false false))
              (:Finished
                (bind _move_curve_end (Timeline|Cube_TL_End PlayFromStart)
                  (:Update
                    (Transformation|SetActorLocation (Math|Vector|MakeVector (.x (Variables|Default|GetGet_Location)) (.y (Variables|Default|GetGet_Location)) (Math|Float|Clamp(Float) (+ (.z (Variables|Default|GetGet_Location)) (* _returnvalue _move_curve_end)) 0.0 (Variables|Default|GetMax_Move))) false false))
                  (:Finished
                    (Variables|Default|SetRun_Animation false)
                    (Variables|/Script/Engine.PrimitiveComponent|SetCanCharacterStepUpOn (Variables|Default|GetBox_Col) "ECB_Yes")))))))))))

(event EventCubeHitEnemy
  (params (HItCube :type Actor%20Object%20Reference) (Hit_Enemy :type Boolean))
  ;[0.15 0.15 0.15 0.5] ヒットストップ
  (Variables|Default|SetCustomTimeDilation (Variables|Default|GetHit%20Stop%20Time%20Dilation))
  (Utilities|FlowControl|Delay (Variables|Default|GetHit%20Stop%20Delay))
  (Variables|Default|SetCustomTimeDilation 1.0))

(fn ConstructionScript)