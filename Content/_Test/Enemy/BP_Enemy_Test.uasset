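; Test enemy character that reacts to being hit by a cube with knockback and hit stop.
; CubeHitEnemy launches it away from the cube with randomized strength, scaling horizontal direction by the vertical component to force diagonal flight, and draws a debug arrow.
; It then briefly changes its own time dilation, using settings read from BP_Default_Setting.
; A DoOnce blocks repeat hits until the delays end; the capsule radius multiplier is currently 1.0.
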(event EventBeginPlay
  (Utilities|FlowControl|Sequence
    (:then_0
      (bind _returnvalue (Actor|GetActorOfClass "/Game/_Test/BP_Default_Setting.BP_Default_Setting_C"))
      (Variables|Default|SetHit%20Stop%20Time%20Dilation (Variables|/Game/_Test/BP_Default_Setting.BP_Default_Setting_C|GetHitStop_TimeDilation _returnvalue))
      (Variables|Default|SetHit%20Stop%20Delay (Variables|/Game/_Test/BP_Default_Setting.BP_Default_Setting_C|GetHitStopDelay _returnvalue)))
    (:then_1
      (Variables|Default|SetCapsule%20Radius (Variables|/Script/Engine.CapsuleComponent|GetCapsuleRadius (Variables|Collision|GetCapsuleComponent))))))

(event EventCubeHitEnemy
  (params (HItCube :type Actor%20Object%20Reference) (Hit_Enemy :type Boolean))
  (bind _returnvalue (Math|Random|RandomFloatinRange 1.0 2.0))
  (bind _returnvalue_2 (Transformation|GetActorLocation HItCube))
  (bind _returnvalue_3 (Transformation|GetActorLocation))
  (bind _knockback_power (Variables|Default|GetKnockBack_Power))
  (bind _returnvalue_4 (Math|Rotator|FindLookatRotation _returnvalue_2 _returnvalue_3))
  (bind _returnvalue_5 (Math|Vector|GetForwardVector _returnvalue_4))
  (bind _returnvalue_6 (* (.z _returnvalue_5) 3.0))
  (bind _returnvalue_7 (* (.y _returnvalue_5) _returnvalue_6))
  (bind _returnvalue_8 (* (.x _returnvalue_5) _returnvalue_6))
  (bind _returnvalue_9 (Math|Vector|MakeVector _returnvalue_8 _returnvalue_7 (.z _returnvalue_5)))
  (bind _returnvalue_10 (* _returnvalue_9 (Math|Vector|MakeVector _knockback_power _knockback_power _knockback_power)))
  (Utilities|FlowControl|DoOnce false :!label _label
    (:Completed
      (Components|Capsule|SetCapsuleRadius (Variables|Collision|GetCapsuleComponent) (* (Variables|Default|GetCapsule%20Radius) 1.0) true)
      (Rendering|Debug|DrawDebugArrow :LineStart _returnvalue_2 :LineEnd (+ _returnvalue_2 _returnvalue_10) :ArrowSize 5.0 :Duration 5.0)
      (Character|LaunchCharacter (* _returnvalue_10 (Math|Vector|MakeVector _returnvalue _returnvalue _returnvalue)) true true) ; 放射状に飛ぶ
      ;[0.15 0.15 0.15 0.5] ヒットストップ
      (Variables|Default|SetCustomTimeDilation (Variables|Default|GetHit%20Stop%20Time%20Dilation))
      (Utilities|FlowControl|Delay (Variables|Default|GetHit%20Stop%20Delay))
      (Variables|Default|SetCustomTimeDilation 1.0)
      (Utilities|FlowControl|Delay 0.1)
      (Components|Capsule|SetCapsuleRadius (Variables|Collision|GetCapsuleComponent) (Variables|Default|GetCapsule%20Radius) true)
      (goto _label Reset))))

(fn ConstructionScript)