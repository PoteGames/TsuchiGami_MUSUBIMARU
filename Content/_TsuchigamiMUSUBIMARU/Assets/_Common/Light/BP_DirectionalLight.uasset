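; Directional light actor Blueprint that publishes its direction and color to the MPC_BaseShader material parameter collection.
; Each Tick writes its forward vector to LightVector and the light component's color to LightColor, so materials reading the collection follow the light at runtime.
; The construction script makes the same writes, keeping the collection in sync when the actor is constructed or edited.
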(event EventBeginPlay)

(event EventTick
  (params (DeltaSeconds :type Float%20%28single-precision%29))
  (Rendering|Material|SetVectorParameterValue "/Game/_TsuchigamiMUSUBIMARU/Assets/_Common/Material/MPC_BaseShader.MPC_BaseShader" "LightVector" (Math|Conversions|ToLinearColor(Vector) (Transformation|GetActorForwardVector)) :!class /Script/Engine.KismetMaterialLibrary)
  (Rendering|Material|SetVectorParameterValue "/Game/_TsuchigamiMUSUBIMARU/Assets/_Common/Material/MPC_BaseShader.MPC_BaseShader" "LightColor" (Rendering|Components|Light|GetLightColor (Variables|Default|GetLightComponent)) :!class /Script/Engine.KismetMaterialLibrary))

(fn ConstructionScript
  (Rendering|Material|SetVectorParameterValue "/Game/_TsuchigamiMUSUBIMARU/Assets/_Common/Material/MPC_BaseShader.MPC_BaseShader" "LightVector" (Math|Conversions|ToLinearColor(Vector) (Transformation|GetActorForwardVector)) :!class /Script/Engine.KismetMaterialLibrary)
  (Rendering|Material|SetVectorParameterValue "/Game/_TsuchigamiMUSUBIMARU/Assets/_Common/Material/MPC_BaseShader.MPC_BaseShader" "LightColor" (Rendering|Components|Light|GetLightColor (Variables|Default|GetLightComponent)) :!class /Script/Engine.KismetMaterialLibrary))